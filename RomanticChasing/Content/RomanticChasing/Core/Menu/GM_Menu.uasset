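; GM_Menu is the game mode for the main menu, connecting the player to Photon Cloud on startup.
; On begin play it sets the device ID as the Photon user ID, binds to connection state changes, connects, and shows a loading screen with the mouse cursor visible.
; When the state becomes Joined Lobby Room, it removes the loading screen and adds the WB_Menu widget to the viewport.
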(event `self.ReceiveBeginPlay`
  (bind _photon_cloud_api (`/Game/RomanticChasing/Core/Library/FL_RomanticFunctions.Get Photon Cloud API`))
  (set `PhotonCloudConfig.userID` (`KismetSystemLibrary.GetDeviceId`) (`PhotonCloudObject.GetPhotonCloudConfig` _photon_cloud_api))
  (add `PhotonCloudObject.OnPhotonCloudStateChanged` _photon_cloud_api (`|CreateDelegate` :!event `on State Change`))
  (`PhotonCloudObject.Connect` (`/Game/RomanticChasing/Core/Library/FL_RomanticFunctions.Get Photon Cloud API`))
  (`/Game/RomanticChasing/Core/Library/FL_RomanticFunctions.Create Loading Screen`)
  (`/Game/RomanticChasing/Core/Library/FL_RomanticFunctions.Set Loading Stats` "連線中...")
  (set `PlayerController.bShowMouseCursor` true (`GameplayStatics.GetPlayerController` 0)))

(event `on State Change`
  (params (NewState :type "EPhotonCloudStates Enum" :default "UNINITIALIZED"))
  (switch `EPhotonCloudStates` NewState
    (:`JOINEDLOBBY`
      (`/Game/RomanticChasing/Core/Library/FL_RomanticFunctions.Remove Loading Screen`)
      (bind _returnvalue (`|CreateWidget` "/Game/RomanticChasing/Widget/Menu/WB_Menu.WB_Menu_C"))
      (`UserWidget.AddToViewport` _returnvalue 0))))

(fn `UserConstructionScript`)